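; Throwable box projectile from a spring puzzle that switches its cube to physics simulation on hit and can be picked up again.
; A Box overlap registers or unregisters it as interactable with the overlapping cast actor.
; Interacting destroys the box and sets PickedUpBox on BigCharacterRef unless one is already held, printing either result.
; The begin overlap sets BigCharacterRef to None, although pickup depends on that reference.
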(event OnComponentBeginOverlap(Box)
  (params (OverlappedComponent :type Primitive%20Component%20Object%20Reference) (OtherActor :type Actor%20Object%20Reference) (OtherComp :type Primitive%20Component%20Object%20Reference) (OtherBodyIndex :type Integer) (bFromSweep :type Boolean) (SweepResult :type Hit%20Result%20Structure%20%28by%20ref%29))
  (bind _asbp_big_character (Utilities|Casting|CastTo OtherActor))
  (CallFunction|UpdateInteract _asbp_big_character self true)
  (Variables|Default|SetBigCharacterRef 0 _asbp_big_character))

(event OnComponentEndOverlap(Box)
  (params (OverlappedComponent :type Primitive%20Component%20Object%20Reference) (OtherActor :type Actor%20Object%20Reference) (OtherComp :type Primitive%20Component%20Object%20Reference) (OtherBodyIndex :type Integer))
  (bind _asbp_big_character (Utilities|Casting|CastTo OtherActor))
  (CallFunction|UpdateInteract _asbp_big_character self false))

(event Custom|DoInteract_1
  (if (Variables|Default|GetPickedUpBox (.BigCharacterRef (Variables|Default|GetBigCharacterRef)))
    (Development|PrintString "Error: Character already has a box picked up" true true "(R=1.000000,G=0.000000,B=0.031819,A=1.000000)" 4.0)
    (else
      (Actor|DestroyActor)
      (Variables|Default|SetPickedUpBox (.BigCharacterRef (Variables|Default|GetBigCharacterRef)) true)
      (Development|PrintString "Box picked up!" true true "(R=0.000000,G=1.000000,B=0.043410,A=1.000000)" 4.0))))

(event EventBeginPlay)

(event Collision|EventHit
  (params (MyComp :type Primitive%20Component%20Object%20Reference) (Other :type Actor%20Object%20Reference) (OtherComp :type Primitive%20Component%20Object%20Reference) (bSelfMoved :type Boolean) (HitLocation :type Vector :default "0, 0, 0") (HitNormal :type Vector :default "0, 0, 0") (NormalImpulse :type Vector :default "0, 0, 0") (Hit :type Hit%20Result%20Structure%20%28by%20ref%29))
  (Physics|SetSimulatePhysics (Variables|Default|GetCube) true))

(fn ConstructionScript)