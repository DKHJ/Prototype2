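; Playable small character that can interact with objects and can itself be picked up by the big character.
; UpdateInteract stores the current target, and the Interact input sends that target an interface interact message.
; Its overlap sphere registers it as the big character's interact target; being interacted with destroys it and sets PickedUpPlayer on that character.
; Debug key 2 possesses the big character.
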(event OnComponentBeginOverlap(Sphere)
  (params (OverlappedComponent :type Primitive%20Component%20Object%20Reference) (OtherActor :type Actor%20Object%20Reference) (OtherComp :type Primitive%20Component%20Object%20Reference) (OtherBodyIndex :type Integer) (bFromSweep :type Boolean) (SweepResult :type Hit%20Result%20Structure%20%28by%20ref%29))
  ;[1 1 1] When we overlap with the big character, update interact
  (bind _asbp_big_character (Utilities|Casting|CastToBP_BigCharacter OtherActor))
  (Default|UpdateInteract _asbp_big_character self true))

(event OnComponentEndOverlap(Sphere)
  (params (OverlappedComponent :type Primitive%20Component%20Object%20Reference) (OtherActor :type Actor%20Object%20Reference) (OtherComp :type Primitive%20Component%20Object%20Reference) (OtherBodyIndex :type Integer))
  ;[1 1 1] When we overlap with the big character, update interact
  (bind _asbp_big_character (Utilities|Casting|CastToBP_BigCharacter OtherActor))
  (Default|UpdateInteract _asbp_big_character self false))

(event EventTick
  (params (DeltaSeconds :type Float%20%28single-precision%29))
  ;[1 1 1] Event Tick, Debug
)

(event EventDoInteract
  ;[1 1 1] Function Interface -> Do Interact -> Destroy ourselves
  (Actor|DestroyActor)
  (Variables|/Game/Characters/Players/BigCharacter/BP_BigCharacter.BP_BigCharacter_C|SetPickedUpPlayer (Variables|Default|GetBigCharacterReference) true))

(event EventBeginPlay
  ;[1 1 1] Begin Play, get big character reference
  (CallFunction|GetBigCharacterReference)
  (Variables|/Game/Characters/Players/BigCharacter/BP_BigCharacter.BP_BigCharacter_C|SetPickedUpPlayer (Variables|Default|GetBigCharacterReference) false))

(event Input|ActionEvents|InputActionInteract
  (params (Key :type Key%20Structure :default "None"))
  (bind _interactactor (Variables|Default|GetInteractActor))
  ;[0 0.9162 1] Interact Event ( Keyboard E or Controller X  )
  (:Pressed
    (if (Variables|Default|GetCanInteract)
      (Development|PrintString (Utilities|String|Append "Interact with: " (Utilities|GetDisplayName _interactactor)))
      (Class|Interact|DoInteract(Message) _interactactor))))

(event Input|KeyboardEvents|2
  (params (Key :type Key%20Structure :default "None"))
  ;[1 0 0.7804] DEBUG: When we press 2 switch the controller back to the big character
  (:Pressed
    (bind _outactors (Actor|GetAllActorsOfClass "/Game/Characters/Players/BigCharacter/BP_BigCharacter.BP_BigCharacter_C"))
    (Pawn|Possess (Game|GetPlayerController 0) (Utilities|Array|Get(acopy) _outactors))))

(fn ConstructionScript)

(fn RotateDebugText)

(fn GetBigCharacterReference
  (bind _outactors (Actor|GetAllActorsOfClass "/Game/Characters/Players/BigCharacter/BP_BigCharacter.BP_BigCharacter_C"))
  (Variables|Default|SetBigCharacterReference (Utilities|Array|Get(acopy) _outactors)))

(fn UpdateInteract
  (params (InteractActor :type Actor%20Object%20Reference) (CanInteract? :type Boolean))
  (bind _output_get (Variables|Default|SetInteractActor InteractActor))
  (bind _output_get_2 (Variables|Default|SetCanInteract CanInteract?))
  (Development|PrintString (Utilities|String|Append (Utilities|String|ToString(Boolean) _output_get_2) " interact with: " (Utilities|GetDisplayName _output_get))))