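; ThrowPlayerProjectile is a projectile that delivers the player at controller index 1 into the world as a small character.
; On BeginPlay it becomes that controller's view target, so the player's camera follows the projectile.
; On Hit it spawns BP_SmallCharacter at Sphere1's location if collision allows, has that controller possess it, then destroys itself.
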(event EventBeginPlay
  (Game|Player|SetViewTargetwithBlend (Game|GetPlayerController 1) self 0.0 "VTBlend_Linear" 0.0 false))

(event Collision|EventHit
  (params (MyComp :type Primitive%20Component%20Object%20Reference) (Other :type Actor%20Object%20Reference) (OtherComp :type Primitive%20Component%20Object%20Reference) (bSelfMoved :type Boolean) (HitLocation :type Vector :default "0, 0, 0") (HitNormal :type Vector :default "0, 0, 0") (NormalImpulse :type Vector :default "0, 0, 0") (Hit :type Hit%20Result%20Structure%20%28by%20ref%29))
  (Development|PrintString "Spawn Little Dude")
  (bind _returnvalue (Game|SpawnActorfromClass "/Game/Characters/Players/SmallCharacter/BP_SmallCharacter.BP_SmallCharacter_C" (Math|Conversions|ToTransform(Vector) (Transformation|GetWorldLocation (Variables|Default|GetSphere1))) "AdjustIfPossibleButDontSpawnIfColliding" 0 0))
  (Pawn|Possess (Game|GetPlayerController 1) _returnvalue)
  (Actor|DestroyActor) ; Then destroy this projectile
)

(fn ConstructionScript)