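; Game mode for local two-player play that spawns a big and a small character, each possessed by its own player controller.
; On BeginPlay it gathers the level's PlayerStart actors and takes the first two as spawn points, using their location only.
; Player controller 0 possesses the big character, then a second local player is created at runtime to possess the small one.
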(event EventBeginPlay
  (CallFunction|GetPlayerStarts)
  (CallFunction|SpawnPlayers))

(fn ConstructionScript)

(fn GetPlayerStarts
  (bind _outactors (Actor|GetAllActorsOfClass "/Script/Engine.PlayerStart"))
  (bind _output_get (Variables|Default|SetPlayerStarts _outactors))
  (Variables|Default|SetPlayerStart1 (Utilities|Array|Get(acopy) _output_get))
  (Variables|Default|SetPlayerStart2 (Utilities|Array|Get(acopy) _output_get 1)))

(fn SpawnPlayers
  (Utilities|FlowControl|Sequence
    (:then_0
      ;[0 0.8924 1] Assign Player Controller 0 to the BigCharacter
      (bind _returnvalue (Game|SpawnActorfromClass "/Game/Characters/Players/BigCharacter/BP_BigCharacter.BP_BigCharacter_C" (Math|Conversions|ToTransform(Vector) (Transformation|GetActorLocation (Variables|Default|GetPlayerStart1))) "Undefined" 0 0))
      (Pawn|Possess (Game|GetPlayerController 0) _returnvalue))
    (:then_1
      ;[0 0.8924 1] Create a player controller and spawn the Small Character
      (bind _returnvalue_2 (Class|GameplayStatics|CreatePlayer 1))
      (bind _returnvalue_3 (Game|SpawnActorfromClass "/Game/Characters/Players/SmallCharacter/BP_SmallCharacter.BP_SmallCharacter_C" (Math|Conversions|ToTransform(Vector) (Transformation|GetActorLocation (Variables|Default|GetPlayerStart2))) "Undefined" _returnvalue_2 0))
      (Pawn|Possess _returnvalue_2 _returnvalue_3))))