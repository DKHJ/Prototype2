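; BP_Puzzle3Box is a puzzle box whose cube slides across linked puzzle piece nodes until a move is blocked.
; BeginPlay snaps the cube to the current piece and triggers MoveLeft.
; MoveLeft and MoveUp walk neighbor links to the last open node, then DoMovement lerps the cube there on a timeline.
; MoveDown teleports node by node, while MoveRight clears the current piece on success and never moves the cube.
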(event Custom|DoMovement
  (params (StartNode :type BP%20Puzzle%20Floor%20Object%20Reference) (EndNode :type BP%20Puzzle%20Floor%20Object%20Reference))
  (bind _returnvalue (Transformation|GetActorLocation EndNode))
  (bind _returnvalue_2 (Transformation|GetActorLocation StartNode))
  (bind _time (Timeline|Timeline_0 PlayFromStart)
    (:Update
      (Transformation|SetWorldLocation (Variables|Default|GetCube) (Math|Vector|MakeVector (Math|Float|Lerp (.x _returnvalue_2) (.x _returnvalue) _time) (Math|Float|Lerp (.y _returnvalue_2) (.y _returnvalue) _time) 8e+01) false false))))

(event Custom|MoveLeft
  ;[0 0.9364 1] Move Left Event
  (Variables|Default|SetBeginNode (Variables|Default|GetCurrentPuzzlePiece))
  (Utilities|FlowControl|ForLoopwithBreak (Variables|/Game/BP_PuzzleFloor.BP_PuzzleFloor_C|GetRowIndex (Variables|Default|GetCurrentPuzzlePiece)) 5 :!label _label
    (:LoopBody
      (bind _canmove (Default|TryMoveLeft (Variables|Default|GetCurrentPuzzlePiece)))
      (if _canmove
        (Variables|Default|SetCurrentPuzzlePiece (Variables|/Game/BP_PuzzleFloor.BP_PuzzleFloor_C|GetNextLeftNode (Variables|Default|GetCurrentPuzzlePiece)))
        (else
          (goto _label Break))))
    (:Completed
      (CallFunction|DoMovement (Variables|Default|GetBeginNode) (Variables|Default|GetCurrentPuzzlePiece)))))

(event Custom|MoveUp
  (Variables|Default|SetBeginNode (Variables|Default|GetCurrentPuzzlePiece))
  (Utilities|FlowControl|ForLoopwithBreak (Variables|/Game/BP_PuzzleFloor.BP_PuzzleFloor_C|GetColumnIndex (Variables|Default|GetCurrentPuzzlePiece)) 5 :!label _label
    (:LoopBody
      (Utilities|IsValid (Variables|/Game/BP_PuzzleFloor.BP_PuzzleFloor_C|GetNextUpNode (Variables|Default|GetCurrentPuzzlePiece))
        (:Is%20Valid
          (bind _canmove (Default|TryMoveUp (Variables|Default|GetCurrentPuzzlePiece)))
          (if _canmove
            (Variables|Default|SetCurrentPuzzlePiece (Variables|/Game/BP_PuzzleFloor.BP_PuzzleFloor_C|GetNextUpNode (Variables|Default|GetCurrentPuzzlePiece)))
            (else
              (goto _label Break))))
        (:Is%20Not%20Valid
          (goto _label Break))))
    (:Completed
      (CallFunction|DoMovement (Variables|Default|GetBeginNode) (Variables|Default|GetCurrentPuzzlePiece)))))

(event Custom|MoveDown
  (Utilities|FlowControl|ForLoopwithBreak (Variables|/Game/BP_PuzzleFloor.BP_PuzzleFloor_C|GetColumnIndex (Variables|Default|GetCurrentPuzzlePiece)) 12 :!label _label
    (:LoopBody
      (Utilities|IsValid (Variables|/Game/BP_PuzzleFloor.BP_PuzzleFloor_C|GetNextDownNode (Variables|Default|GetCurrentPuzzlePiece))
        (:Is%20Valid
          (bind _canmove (Default|TryMoveDown (Variables|Default|GetCurrentPuzzlePiece)))
          (if _canmove
            (Transformation|SetWorldLocation (Variables|Default|GetCube) (Math|Vector|MakeVector (.x (Transformation|GetActorLocation (Variables|/Game/BP_PuzzleFloor.BP_PuzzleFloor_C|GetNextDownNode (Variables|Default|GetCurrentPuzzlePiece)))) (.y (Transformation|GetActorLocation (Variables|/Game/BP_PuzzleFloor.BP_PuzzleFloor_C|GetNextDownNode (Variables|Default|GetCurrentPuzzlePiece)))) 8e+01) false false)
            (Variables|Default|SetCurrentPuzzlePiece (Variables|/Game/BP_PuzzleFloor.BP_PuzzleFloor_C|GetNextDownNode (Variables|Default|GetCurrentPuzzlePiece)))
            (else
              (goto _label Break))))
        (:Is%20Not%20Valid
          (goto _label Break))))))

(event Custom|MoveRight
  (Variables|Default|SetBeginNode (Variables|Default|GetCurrentPuzzlePiece))
  (Utilities|FlowControl|ForLoopwithBreak (Variables|/Game/BP_PuzzleFloor.BP_PuzzleFloor_C|GetRowIndex (Variables|Default|GetCurrentPuzzlePiece)) 12 :!label _label
    (:LoopBody
      (Utilities|IsValid (Variables|/Game/BP_PuzzleFloor.BP_PuzzleFloor_C|GetNextRightNode (Variables|Default|GetCurrentPuzzlePiece))
        (:Is%20Valid
          (bind _canmove (Default|TryMoveRight (Variables|Default|GetCurrentPuzzlePiece)))
          (if _canmove
            (Variables|Default|SetCurrentPuzzlePiece 0)
            (else
              (goto _label Break))))
        (:Is%20Not%20Valid
          (goto _label Break))))))

(event EventBeginPlay
  (bind _currentpuzzlepiece (Variables|Default|GetCurrentPuzzlePiece))
  (bind _returnvalue (Transformation|GetActorLocation _currentpuzzlepiece))
  (Transformation|SetWorldLocation (Variables|Default|GetCube) (Math|Vector|MakeVector (.x _returnvalue) (.y _returnvalue) 8e+01) false false)
  (CallFunction|MoveLeft))

(fn ConstructionScript)