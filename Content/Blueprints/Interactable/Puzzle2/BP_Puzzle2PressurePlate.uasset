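; Pressure plate interactable for Puzzle 2 that responds only to BP_SmallCharacter entering or leaving its collision box.
; Overlap sets the Activated state, which plays or reverses a timeline that slides the button along a spline using its length.
; Each timeline update also calls DoInteract on the referenced PlatformMove2Ref, so the linked platform is triggered repeatedly while the button moves, not once per press.
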(event OnComponentBeginOverlap(CollisionBox)
  (params (OverlappedComponent :type Primitive%20Component%20Object%20Reference) (OtherActor :type Actor%20Object%20Reference) (OtherComp :type Primitive%20Component%20Object%20Reference) (OtherBodyIndex :type Integer) (bFromSweep :type Boolean) (SweepResult :type Hit%20Result%20Structure%20%28by%20ref%29))
  ;[0 0.8689 1] Collision Overlaps
  (Utilities|Casting|CastToBP_SmallCharacter OtherActor)
  (Development|PrintString "Pressure plate Activated!")
  (Variables|InteractSettings|SetActivated? true)
  (CallFunction|DoInteract))

(event OnComponentEndOverlap(CollisionBox)
  (params (OverlappedComponent :type Primitive%20Component%20Object%20Reference) (OtherActor :type Actor%20Object%20Reference) (OtherComp :type Primitive%20Component%20Object%20Reference) (OtherBodyIndex :type Integer))
  ;[0 0.8689 1] Collision Overlaps
  (Utilities|Casting|CastToBP_SmallCharacter OtherActor)
  (if true
    (Development|PrintString "Pressure plate Deactivated!")
    (Variables|InteractSettings|SetActivated? false)
    (CallFunction|DoInteract)))

(event EventDoInteract
  (if (Variables|InteractSettings|GetActivated?)
    ;[0 1 1] Move the button down
    (bind _time (Timeline|Timeline Play)
      (:Update
        (Transformation|SetWorldLocation (Variables|Default|GetButton) (Spline|GetLocationatDistanceAlongSpline (Variables|Default|GetSpline) (* _time (Spline|GetSplineLength (Variables|Default|GetSpline))) "World") false false)
        (Default|DoInteract (Variables|InteractSettings|GetPlatformMove2Ref))))
    (else
      (Timeline|Timeline Reverse))))

(fn ConstructionScript)