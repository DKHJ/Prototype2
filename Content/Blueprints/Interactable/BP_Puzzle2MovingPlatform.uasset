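; Puzzle 2 moving platform that carries its mesh along a spline, either automatically or toggled through interaction.
; DoInteract flips the activated state, then Activate waits a configurable delay and plays or reverses the movement timeline.
; The timeline's normalized distance, scaled by spline length, sets the mesh's world location without sweeping.
; In automatic mode it starts on BeginPlay and flips direction whenever the timeline finishes, looping back and forth.
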(event Custom|Activate
  (Utilities|FlowControl|Delay (Variables|PlatformSettings|GetAutomaticDelay))
  (if (Variables|PlatformSettings|GetIsActivated?)
    (bind _distance (Timeline|MovementTimeline Play)
      (:Update
        (Transformation|SetWorldLocation (Variables|Default|GetPlatformMesh) (Spline|GetLocationatDistanceAlongSpline (Variables|Default|GetSpline) (* _distance (Spline|GetSplineLength (Variables|Default|GetSpline))) "World") false false))
      (:Finished
        (if (Variables|PlatformSettings|GetIsAutomatic?)
          (if (Variables|PlatformSettings|GetIsActivated?)
            (Variables|PlatformSettings|SetIsActivated? false)
            (else
              (Variables|PlatformSettings|SetIsActivated? true)))
          (CallFunction|Activate))))
    (else
      (Timeline|MovementTimeline Reverse))))

(event EventDoInteract
  ;[1 1 1] Function Interface event
  (if (Variables|PlatformSettings|GetIsActivated?)
    (Variables|PlatformSettings|SetIsActivated? false)
    (else
      (Variables|PlatformSettings|SetIsActivated? true)))
  (CallFunction|Activate))

(event EventBeginPlay
  ;[1 1 1] BeginPlay, check if we have been set to automatic
  (if (Variables|PlatformSettings|GetIsAutomatic?)
    (Variables|PlatformSettings|SetIsActivated? true)
    (CallFunction|Activate)))

(fn ConstructionScript)