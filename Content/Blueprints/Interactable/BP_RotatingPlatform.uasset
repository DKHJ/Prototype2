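; Interactable platform that swings a quarter turn and back, either on its own or when its events are called.
; Rotate and ReverseRotate set opposite rates on a RotatingMovement component, activate it for a timed one-second window, then deactivate it.
; With Automatic set, BeginPlay starts Rotate and the two events call each other after AutomaticDelay, looping indefinitely.
; The angle comes from rate and delay timing, with no snap to a target rotation.
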(event Custom|Rotate
  (Variables|/Script/Engine.RotatingMovementComponent|SetRotationRate (Variables|Default|GetRotatingMovement) "0, 0,90.000000")
  (Components|Activation|Activate (Variables|Default|GetRotatingMovement) false)
  (Utilities|FlowControl|Delay 1.0)
  (Components|Activation|Deactivate (Variables|Default|GetRotatingMovement))
  (if (Variables|RotateSettings|GetAutomatic?)
    (Utilities|FlowControl|Delay (Variables|RotateSettings|GetAutomaticDelay))
    (CallFunction|ReverseRotate)))

(event Custom|ReverseRotate
  (Variables|/Script/Engine.RotatingMovementComponent|SetRotationRate (Variables|Default|GetRotatingMovement) "0, 0,-90.000000")
  (Components|Activation|Activate (Variables|Default|GetRotatingMovement) false)
  (Utilities|FlowControl|Delay 1.0)
  (Components|Activation|Deactivate (Variables|Default|GetRotatingMovement))
  (if (Variables|RotateSettings|GetAutomatic?)
    (Utilities|FlowControl|Delay (Variables|RotateSettings|GetAutomaticDelay))
    (CallFunction|Rotate)))

(event EventBeginPlay
  (if (Variables|RotateSettings|GetAutomatic?)
    (CallFunction|Rotate)))

(fn ConstructionScript)