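; Interactable moving platform that slides its mesh back and forth along a spline, either automatically or when interacted with.
; The interact event toggles the activated state, which plays or reverses a timeline whose alpha, scaled by spline length, sets the mesh's world location.
; In automatic mode it starts on BeginPlay and flips direction after a delay whenever the timeline finishes.
; Tick shows the activated state through debug text and materials.
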(event Custom|Activate
  (if (Variables|PlatformSettings|GetIsActivated?)
    (bind _distance (Timeline|MovementTimeline Play)
      (:Update
        (Transformation|SetWorldLocation (Variables|Default|GetPlatformMesh) (Spline|GetLocationatDistanceAlongSpline (Variables|Default|GetSpline) (* _distance (Spline|GetSplineLength (Variables|Default|GetSpline))) "World") false false))
      (:Finished
        (if (Variables|PlatformSettings|GetIsAutomatic?)
          (Utilities|FlowControl|Delay (Variables|PlatformSettings|GetAutomaticDelay))
          (if (Variables|PlatformSettings|GetIsActivated?)
            (Variables|PlatformSettings|SetIsActivated? false)
            (else
              (Variables|PlatformSettings|SetIsActivated? true)))
          (CallFunction|Activate))))
    (else
      (Timeline|MovementTimeline Reverse))))

(event EventDoInteract
  ;[1 1 1] Function Interface event
  (if (Variables|PlatformSettings|GetIsActivated?)
    (Variables|PlatformSettings|SetIsActivated? false)
    (else
      (Variables|PlatformSettings|SetIsActivated? true)))
  (CallFunction|Activate))

(event EventTick
  (params (DeltaSeconds :type Float%20%28single-precision%29))
  (Rendering|Components|TextRender|SetText (Variables|Default|GetDebugText) (Utilities|Text|ToText(Boolean) (Variables|PlatformSettings|GetIsActivated?)))
  (if (Variables|PlatformSettings|GetIsActivated?)
    (Rendering|Material|SetMaterial (Variables|Default|GetPlatformMesh) 0 "/Game/Assets/Materials/DEBUG_TRUE.DEBUG_TRUE")
    (else
      (Rendering|Material|SetMaterial (Variables|Default|GetPlatformMesh) 0 "/Game/Assets/Materials/DEBUG_FALSE.DEBUG_FALSE"))))

(event EventBeginPlay
  ;[1 1 1] BeginPlay, check if we have been set to automatic
  (if (Variables|PlatformSettings|GetIsAutomatic?)
    (Variables|PlatformSettings|SetIsActivated? true)
    (CallFunction|Activate)))

(fn ConstructionScript)