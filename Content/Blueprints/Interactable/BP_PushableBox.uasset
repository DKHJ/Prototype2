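; BP_PushableBox is an interactable box that only the big character can set free to move.
; Overlaps on the X_Box and Y_Box triggers switch the Cube's physics simulation on when a BP_BigCharacter enters and off when it leaves.
; DoInteract applies a fixed forward-and-up impulse to the Cube, passing the Sphere's relative location as the impulse point.
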(event OnComponentBeginOverlap(Y_Box)
  (params (OverlappedComponent :type Primitive%20Component%20Object%20Reference) (OtherActor :type Actor%20Object%20Reference) (OtherComp :type Primitive%20Component%20Object%20Reference) (OtherBodyIndex :type Integer) (bFromSweep :type Boolean) (SweepResult :type Hit%20Result%20Structure%20%28by%20ref%29))
  ;[0 0.9319 1] Collision Overlaps
  (Utilities|Casting|CastToBP_BigCharacter OtherActor)
  (Physics|SetSimulatePhysics (Variables|Default|GetCube) true))

(event OnComponentEndOverlap(Y_Box)
  (params (OverlappedComponent :type Primitive%20Component%20Object%20Reference) (OtherActor :type Actor%20Object%20Reference) (OtherComp :type Primitive%20Component%20Object%20Reference) (OtherBodyIndex :type Integer))
  ;[0 0.9319 1] Collision Overlaps
  (Utilities|Casting|CastToBP_BigCharacter OtherActor)
  (Physics|SetSimulatePhysics (Variables|Default|GetCube) false))

(event OnComponentBeginOverlap(X_Box)
  (params (OverlappedComponent :type Primitive%20Component%20Object%20Reference) (OtherActor :type Actor%20Object%20Reference) (OtherComp :type Primitive%20Component%20Object%20Reference) (OtherBodyIndex :type Integer) (bFromSweep :type Boolean) (SweepResult :type Hit%20Result%20Structure%20%28by%20ref%29))
  ;[0 0.9319 1] Collision Overlaps
  (Utilities|Casting|CastToBP_BigCharacter OtherActor)
  (Physics|SetSimulatePhysics (Variables|Default|GetCube) true))

(event OnComponentEndOverlap(X_Box)
  (params (OverlappedComponent :type Primitive%20Component%20Object%20Reference) (OtherActor :type Actor%20Object%20Reference) (OtherComp :type Primitive%20Component%20Object%20Reference) (OtherBodyIndex :type Integer))
  ;[0 0.9319 1] Collision Overlaps
  (Utilities|Casting|CastToBP_BigCharacter OtherActor)
  (Physics|SetSimulatePhysics (Variables|Default|GetCube) false))

(event Custom|Impulse
  (Physics|AddImpulseatLocation (Variables|Default|GetCube) "170000.000000,0.000000,100000.000000" (Variables|/Script/Engine.SceneComponent|GetRelativeLocation (Variables|Default|GetSphere)) "None"))

(event EventDoInteract
  (CallFunction|Impulse))

(fn ConstructionScript)