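; MapBoundary is an interactable boundary that responds to characters and thrown projectiles overlapping its collision component.
; A cast chain sends teleports to TeleportTargetLocation, but as wired, the BP_BigCharacter branch targets the small-character cast result.
; The BP_SmallCharacter and ThrowPlayerProjectile branches call Teleport on the boundary itself rather than the overlapping actor.
; A ThrowBoxProjectile is destroyed and replaced by a double-scale one at BoxTeleportLocation.
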(event OnComponentBeginOverlap(CollisionComponent)
  (params (OverlappedComponent :type Primitive%20Component%20Object%20Reference) (OtherActor :type Actor%20Object%20Reference) (OtherComp :type Primitive%20Component%20Object%20Reference) (OtherBodyIndex :type Integer) (bFromSweep :type Boolean) (SweepResult :type Hit%20Result%20Structure%20%28by%20ref%29))
  (Utilities|Casting|CastToBP_BigCharacter OtherActor
    (:then
      (Transformation|Teleport (stale _asbp_small_character) (Transformation|GetActorLocation (Variables|Default|GetTeleportTargetLocation)) "0, 0, 0"))
    (:CastFailed
      (bind _asbp_small_character (Utilities|Casting|CastToBP_SmallCharacter OtherActor)
        (:then
          (Transformation|Teleport (Transformation|GetActorLocation (Variables|Default|GetTeleportTargetLocation)) "0, 0, 0"))
        (:CastFailed
          (Utilities|Casting|CastToThrowPlayerProjectile OtherActor
            (:then
              (Transformation|Teleport (Transformation|GetActorLocation (Variables|Default|GetTeleportTargetLocation)) "0, 0, 0"))
            (:CastFailed
              (bind _asthrow_box_projectile (Utilities|Casting|CastToThrowBoxProjectile OtherActor))
              (Actor|DestroyActor _asthrow_box_projectile)
              (Game|SpawnActorfromClass "/Game/Blueprints/Interactable/Puzzle2/ThrowBoxProjectile.ThrowBoxProjectile_C" (Math|Transform|MakeTransform (Transformation|GetActorLocation (Variables|Default|GetBoxTeleportLocation)) "0, 0, 0" "2.000000,2.000000,2.000000") "Undefined" 0 0))))))))

(fn ConstructionScript)