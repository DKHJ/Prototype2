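; Pushable box for puzzle 3 that slides across a grid of linked puzzle-piece nodes until it can go no further.
; Four side collision volumes set the push direction and register the box as BP_BigCharacter's interact target.
; DoInteract dispatches to a Move event that walks neighbor nodes while TryMove succeeds, within loop bounds based on row or column index.
; A timeline then lerps the cube from start node to end node at fixed height.
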(event OnComponentBeginOverlap(MoveUpCollision)
  (params (OverlappedComponent :type Primitive%20Component%20Object%20Reference) (OtherActor :type Actor%20Object%20Reference) (OtherComp :type Primitive%20Component%20Object%20Reference) (OtherBodyIndex :type Integer) (bFromSweep :type Boolean) (SweepResult :type Hit%20Result%20Structure%20%28by%20ref%29))
  (bind _asbp_big_character (Utilities|Casting|CastToBP_BigCharacter OtherActor))
  (Default|UpdateInteract _asbp_big_character self true)
  (Variables|Default|SetDirection "UP"))

(event OnComponentEndOverlap(MoveUpCollision)
  (params (OverlappedComponent :type Primitive%20Component%20Object%20Reference) (OtherActor :type Actor%20Object%20Reference) (OtherComp :type Primitive%20Component%20Object%20Reference) (OtherBodyIndex :type Integer))
  (bind _asbp_big_character (Utilities|Casting|CastToBP_BigCharacter OtherActor))
  (Default|UpdateInteract _asbp_big_character self false)
  (Variables|Default|SetDirection "NONE"))

(event OnComponentBeginOverlap(MoveDownCollision)
  (params (OverlappedComponent :type Primitive%20Component%20Object%20Reference) (OtherActor :type Actor%20Object%20Reference) (OtherComp :type Primitive%20Component%20Object%20Reference) (OtherBodyIndex :type Integer) (bFromSweep :type Boolean) (SweepResult :type Hit%20Result%20Structure%20%28by%20ref%29))
  (bind _asbp_big_character (Utilities|Casting|CastToBP_BigCharacter OtherActor))
  (Default|UpdateInteract _asbp_big_character self true)
  (Variables|Default|SetDirection "DOWN"))

(event OnComponentEndOverlap(MoveDownCollision)
  (params (OverlappedComponent :type Primitive%20Component%20Object%20Reference) (OtherActor :type Actor%20Object%20Reference) (OtherComp :type Primitive%20Component%20Object%20Reference) (OtherBodyIndex :type Integer))
  (bind _asbp_big_character (Utilities|Casting|CastToBP_BigCharacter OtherActor))
  (Default|UpdateInteract _asbp_big_character self false)
  (Variables|Default|SetDirection "NONE"))

(event OnComponentBeginOverlap(MoveLeftCollision)
  (params (OverlappedComponent :type Primitive%20Component%20Object%20Reference) (OtherActor :type Actor%20Object%20Reference) (OtherComp :type Primitive%20Component%20Object%20Reference) (OtherBodyIndex :type Integer) (bFromSweep :type Boolean) (SweepResult :type Hit%20Result%20Structure%20%28by%20ref%29))
  (bind _asbp_big_character (Utilities|Casting|CastToBP_BigCharacter OtherActor))
  (Default|UpdateInteract _asbp_big_character self true)
  (Variables|Default|SetDirection "LEFT"))

(event OnComponentEndOverlap(MoveLeftCollision)
  (params (OverlappedComponent :type Primitive%20Component%20Object%20Reference) (OtherActor :type Actor%20Object%20Reference) (OtherComp :type Primitive%20Component%20Object%20Reference) (OtherBodyIndex :type Integer))
  (bind _asbp_big_character (Utilities|Casting|CastToBP_BigCharacter OtherActor))
  (Default|UpdateInteract _asbp_big_character self false)
  (Variables|Default|SetDirection "NONE"))

(event OnComponentBeginOverlap(MoveRightCollision)
  (params (OverlappedComponent :type Primitive%20Component%20Object%20Reference) (OtherActor :type Actor%20Object%20Reference) (OtherComp :type Primitive%20Component%20Object%20Reference) (OtherBodyIndex :type Integer) (bFromSweep :type Boolean) (SweepResult :type Hit%20Result%20Structure%20%28by%20ref%29))
  (bind _asbp_big_character (Utilities|Casting|CastToBP_BigCharacter OtherActor))
  (Default|UpdateInteract _asbp_big_character self true)
  (Variables|Default|SetDirection "RIGHT"))

(event OnComponentEndOverlap(MoveRightCollision)
  (params (OverlappedComponent :type Primitive%20Component%20Object%20Reference) (OtherActor :type Actor%20Object%20Reference) (OtherComp :type Primitive%20Component%20Object%20Reference) (OtherBodyIndex :type Integer))
  (bind _asbp_big_character (Utilities|Casting|CastToBP_BigCharacter OtherActor))
  (Default|UpdateInteract _asbp_big_character self false)
  (Variables|Default|SetDirection "NONE"))

(event Custom|DoMovement
  (params (StartNode :type BP%20Puzzle%20Floor%20Object%20Reference) (EndNode :type BP%20Puzzle%20Floor%20Object%20Reference))
  (bind _returnvalue (Transformation|GetActorLocation EndNode))
  (bind _returnvalue_2 (Transformation|GetActorLocation StartNode))
  (bind _time (Timeline|Timeline_0 PlayFromStart)
    (:Update
      (Transformation|SetWorldLocation (Variables|Default|GetCube) (Math|Vector|MakeVector (Math|Float|Lerp (.x _returnvalue_2) (.x _returnvalue) _time) (Math|Float|Lerp (.y _returnvalue_2) (.y _returnvalue) _time) 3e+01) false false))))

(event Custom|MoveLeft
  ;[0 0.9364 1] Move Left Event
  (Variables|Default|SetBeginNode (Variables|Default|GetCurrentPuzzlePiece))
  (Utilities|FlowControl|ForLoopwithBreak (Variables|/Game/Blueprints/Interactable/BP_PuzzleFloor.BP_PuzzleFloor_C|GetRowIndex (Variables|Default|GetCurrentPuzzlePiece)) 5 :!label _label
    (:LoopBody
      (bind _canmove (Default|TryMoveLeft (Variables|Default|GetCurrentPuzzlePiece)))
      (if _canmove
        (Variables|Default|SetCurrentPuzzlePiece (Variables|/Game/Blueprints/Interactable/BP_PuzzleFloor.BP_PuzzleFloor_C|GetNextLeftNode (Variables|Default|GetCurrentPuzzlePiece)))
        (else
          (goto _label Break))))
    (:Completed
      (CallFunction|DoMovement (Variables|Default|GetBeginNode) (Variables|Default|GetCurrentPuzzlePiece)))))

(event Custom|MoveUp
  (Variables|Default|SetBeginNode (Variables|Default|GetCurrentPuzzlePiece))
  (Utilities|FlowControl|ForLoopwithBreak (Variables|/Game/Blueprints/Interactable/BP_PuzzleFloor.BP_PuzzleFloor_C|GetColumnIndex (Variables|Default|GetCurrentPuzzlePiece)) 5 :!label _label
    (:LoopBody
      (Utilities|IsValid (Variables|/Game/Blueprints/Interactable/BP_PuzzleFloor.BP_PuzzleFloor_C|GetNextUpNode (Variables|Default|GetCurrentPuzzlePiece))
        (:Is%20Valid
          (bind _canmove (Default|TryMoveUp (Variables|Default|GetCurrentPuzzlePiece)))
          (if _canmove
            (Variables|Default|SetCurrentPuzzlePiece (Variables|/Game/Blueprints/Interactable/BP_PuzzleFloor.BP_PuzzleFloor_C|GetNextUpNode (Variables|Default|GetCurrentPuzzlePiece)))
            (else
              (goto _label Break))))
        (:Is%20Not%20Valid
          (goto _label Break))))
    (:Completed
      (CallFunction|DoMovement (Variables|Default|GetBeginNode) (Variables|Default|GetCurrentPuzzlePiece)))))

(event Custom|MoveDown
  (Variables|Default|SetBeginNode (Variables|Default|GetCurrentPuzzlePiece))
  (Utilities|FlowControl|ForLoopwithBreak (Variables|/Game/Blueprints/Interactable/BP_PuzzleFloor.BP_PuzzleFloor_C|GetColumnIndex (Variables|Default|GetCurrentPuzzlePiece)) 12 :!label _label
    (:LoopBody
      (Utilities|IsValid (Variables|/Game/Blueprints/Interactable/BP_PuzzleFloor.BP_PuzzleFloor_C|GetNextDownNode (Variables|Default|GetCurrentPuzzlePiece))
        (:Is%20Valid
          (bind _canmove (Default|TryMoveDown (Variables|Default|GetCurrentPuzzlePiece)))
          (if _canmove
            (Variables|Default|SetCurrentPuzzlePiece (Variables|/Game/Blueprints/Interactable/BP_PuzzleFloor.BP_PuzzleFloor_C|GetNextDownNode (Variables|Default|GetCurrentPuzzlePiece)))
            (else
              (goto _label Break))))
        (:Is%20Not%20Valid
          (goto _label Break))))
    (:Completed
      (CallFunction|DoMovement (Variables|Default|GetBeginNode) (Variables|Default|GetCurrentPuzzlePiece)))))

(event Custom|MoveRight
  (Variables|Default|SetBeginNode (Variables|Default|GetCurrentPuzzlePiece))
  (Utilities|FlowControl|ForLoopwithBreak (Variables|/Game/Blueprints/Interactable/BP_PuzzleFloor.BP_PuzzleFloor_C|GetRowIndex (Variables|Default|GetCurrentPuzzlePiece)) 12 :!label _label
    (:LoopBody
      (Utilities|IsValid (Variables|/Game/Blueprints/Interactable/BP_PuzzleFloor.BP_PuzzleFloor_C|GetNextRightNode (Variables|Default|GetCurrentPuzzlePiece))
        (:Is%20Valid
          (bind _canmove (Default|TryMoveRight (Variables|Default|GetCurrentPuzzlePiece)))
          (if _canmove
            (Variables|Default|SetCurrentPuzzlePiece (Variables|/Game/Blueprints/Interactable/BP_PuzzleFloor.BP_PuzzleFloor_C|GetNextRightNode (Variables|Default|GetCurrentPuzzlePiece)))
            (else
              (goto _label Break))))
        (:Is%20Not%20Valid
          (goto _label Break))))
    (:Completed
      (CallFunction|DoMovement (Variables|Default|GetBeginNode) (Variables|Default|GetCurrentPuzzlePiece)))))

(event EventBeginPlay
  (bind _currentpuzzlepiece (Variables|Default|GetCurrentPuzzlePiece))
  (bind _returnvalue (Transformation|GetActorLocation _currentpuzzlepiece))
  (Transformation|SetWorldLocation (Variables|Default|GetCube) (Math|Vector|MakeVector (.x _returnvalue) (.y _returnvalue) 3e+01) false false))

(event EventDoInteract
  (switch string (Variables|Default|GetDirection)
    (:UP
      (CallFunction|MoveUp))
    (:DOWN
      (CallFunction|MoveDown))
    (:LEFT
      (CallFunction|MoveLeft))
    (:RIGHT
      (CallFunction|MoveRight))))

(fn ConstructionScript)