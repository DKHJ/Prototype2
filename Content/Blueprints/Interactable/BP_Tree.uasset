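; BP_Tree is an interactable tree that the big character can kick over once.
; Overlapping its box registers the tree with BP_BigCharacter as the interact target and shows a prompt until used.
; DoInteract plays the falling sound, the character's kick montage and the tree's skeletal animation.
; It then swaps collision from the standing base to the fallen shape, sets IsActivated and hides the prompt.
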(event OnComponentBeginOverlap(Box)
  (params (OverlappedComponent :type Primitive%20Component%20Object%20Reference) (OtherActor :type Actor%20Object%20Reference) (OtherComp :type Primitive%20Component%20Object%20Reference) (OtherBodyIndex :type Integer) (bFromSweep :type Boolean) (SweepResult :type Hit%20Result%20Structure%20%28by%20ref%29))
  (bind _asbp_big_character (Utilities|Casting|CastToBP_BigCharacter OtherActor))
  (Default|UpdateInteract _asbp_big_character self true)
  (Variables|Default|SetBigCharRef _asbp_big_character)
  (if (not (Variables|Default|GetIsActivated?))
    (Rendering|SetVisibility (Variables|Default|GetInteractText) true false)))

(event OnComponentEndOverlap(Box)
  (params (OverlappedComponent :type Primitive%20Component%20Object%20Reference) (OtherActor :type Actor%20Object%20Reference) (OtherComp :type Primitive%20Component%20Object%20Reference) (OtherBodyIndex :type Integer))
  (bind _asbp_big_character (Utilities|Casting|CastToBP_BigCharacter OtherActor))
  (Default|UpdateInteract _asbp_big_character self false)
  (if (not (Variables|Default|GetIsActivated?))
    (Rendering|SetVisibility (Variables|Default|GetInteractText) false false)))

(event EventDoInteract
  (if (not (Variables|Default|GetIsActivated?))
    (Audio|PlaySound2D "/Game/Audio/TreeFalling.TreeFalling" 1.0 1.0 0.0 0 0)
    (Animation|PlayAnimMontage (Variables|Default|GetBigCharRef) "/Game/Animations/BigCharacter/Big_KickMont.Big_KickMont" 1.0 "None")
    (Audio|Components|Audio|Play (Variables|Default|GetSkeletalMesh) false)
    (Collision|SetCollisionEnabled (Variables|Default|GetCollisionFallen) "QueryAndPhysics")
    (Collision|SetCollisionEnabled (Variables|Default|GetCollisionBase) "NoCollision")
    (Variables|Default|SetIsActivated? true)
    (Rendering|SetVisibility (Variables|Default|GetInteractText) false false)))

(event EventBeginPlay
  (Collision|SetCollisionEnabled (Variables|Default|GetCollisionFallen) "NoCollision"))

(fn ConstructionScript)