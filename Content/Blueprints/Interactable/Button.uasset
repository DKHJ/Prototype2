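; Interactable button that a BP_BigCharacter can use to trigger a linked moving platform.
; Overlapping its collision box shows or hides the interact text and registers or unregisters the button as the character's current interact target.
; DoInteract prints a debug message and forwards the call to the referenced moving platform; the DoSomething function is an empty stub.
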(event OnComponentBeginOverlap(CollisionBox)
  (params (OverlappedComponent :type Primitive%20Component%20Object%20Reference) (OtherActor :type Actor%20Object%20Reference) (OtherComp :type Primitive%20Component%20Object%20Reference) (OtherBodyIndex :type Integer) (bFromSweep :type Boolean) (SweepResult :type Hit%20Result%20Structure%20%28by%20ref%29))
  (bind _asbp_big_character (Utilities|Casting|CastToBP_BigCharacter OtherActor))
  (Rendering|SetVisibility (Variables|Default|GetInteractText) true false)
  (Default|UpdateInteract _asbp_big_character self true))

(event OnComponentEndOverlap(CollisionBox)
  (params (OverlappedComponent :type Primitive%20Component%20Object%20Reference) (OtherActor :type Actor%20Object%20Reference) (OtherComp :type Primitive%20Component%20Object%20Reference) (OtherBodyIndex :type Integer))
  (bind _asbp_big_character (Utilities|Casting|CastToBP_BigCharacter OtherActor))
  (Rendering|SetVisibility (Variables|Default|GetInteractText) false false)
  (Default|UpdateInteract _asbp_big_character self false))

(event EventDoInteract
  (Development|PrintString "Button should do something now")
  (Default|DoInteract (Variables|Default|GetMovingPlatformReference)))

(fn ConstructionScript)

(fn DoSomething)