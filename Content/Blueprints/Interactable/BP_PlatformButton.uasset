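; BP_PlatformButton is an interactable button that toggles its linked moving platform, with only one button meant to stay active at a time.
; Overlapping BP_BigCharacter shows a prompt and registers the button for interaction.
; DoInteract flips Activated, triggers the platform, then after a short delay resets other active buttons and their platforms via an array gathered at BeginPlay.
; Tick swaps debug materials to show state; construction labels the button number.
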(event OnComponentBeginOverlap(CollisionBox)
  (params (OverlappedComponent :type Primitive%20Component%20Object%20Reference) (OtherActor :type Actor%20Object%20Reference) (OtherComp :type Primitive%20Component%20Object%20Reference) (OtherBodyIndex :type Integer) (bFromSweep :type Boolean) (SweepResult :type Hit%20Result%20Structure%20%28by%20ref%29))
  ;[0 0.8962 1] OverlapEvents
  (bind _asbp_big_character (Utilities|Casting|CastToBP_BigCharacter OtherActor))
  (Rendering|SetVisibility (Variables|Default|GetInteractText) true false)
  (Default|UpdateInteract _asbp_big_character self true))

(event OnComponentEndOverlap(CollisionBox)
  (params (OverlappedComponent :type Primitive%20Component%20Object%20Reference) (OtherActor :type Actor%20Object%20Reference) (OtherComp :type Primitive%20Component%20Object%20Reference) (OtherBodyIndex :type Integer))
  ;[0 0.8962 1] OverlapEvents
  (bind _asbp_big_character (Utilities|Casting|CastToBP_BigCharacter OtherActor))
  (Rendering|SetVisibility (Variables|Default|GetInteractText) false false)
  (Default|UpdateInteract _asbp_big_character self false))

(event EventBeginPlay
  ;[1 1 1] When we are created, add this object into the array and set the count
  (bind _outactors (Actor|GetAllActorsOfClass "BP_PlatformButton_C"))
  (Variables|ButtonInteractions|SetAllButtons _outactors))

(event EventTick
  (params (DeltaSeconds :type Float%20%28single-precision%29))
  (if (Variables|ButtonInteractions|GetActivated?)
    (Rendering|Material|SetMaterial (Variables|Default|GetCube) 0 "/Game/Assets/Materials/DEBUG_TRUE.DEBUG_TRUE")
    (else
      (Rendering|Material|SetMaterial (Variables|Default|GetCube) 0 "/Game/Assets/Materials/DEBUG_FALSE.DEBUG_FALSE"))))

(event EventDoInteract
  (if (Variables|ButtonInteractions|GetActivated?)
    (Variables|ButtonInteractions|SetActivated? false)
    (else
      (Variables|ButtonInteractions|SetActivated? true)))
  (Default|DoInteract (Variables|ButtonInteractions|GetMovingPlatformReference))
  (Utilities|FlowControl|Delay 0.8)
  (CallFunction|ResetAllOtherButtons self))

(fn ConstructionScript
  (Rendering|Components|TextRender|SetText (Variables|Default|GetDebugText) (Utilities|Text|ToText(Integer) (Variables|ButtonInteractions|GetButtonNumber))))

(fn ResetAllButtons
  (Variables|Default|SetResetCount 0)
  (for _array_element (Variables|ButtonInteractions|GetAllButtons)
    (if (Variables|BP_PlatformButton_C|GetActivated? _array_element)
      (Variables|BP_PlatformButton_C|SetActivated? _array_element false)
      (Default|DoInteract (Variables|BP_PlatformButton_C|GetMovingPlatformReference _array_element))
      (Math|Integer|IncrementInt (Variables|Default|GetResetCount))))
  (Development|PrintString (Utilities|String|Append "Reset Loop Completed: Reset count = " (Utilities|String|ToString(Integer) (Variables|Default|GetResetCount)))))

(fn ResetAllOtherButtons
  (params (CurrentButton :type BP%20Platform%20Button%20Object%20Reference))
  (Variables|Default|SetResetCount 0)
  (for _array_element (Variables|ButtonInteractions|GetAllButtons)
    (if (not (== _array_element CurrentButton))
      (if (Variables|BP_PlatformButton_C|GetActivated? _array_element)
        (Variables|BP_PlatformButton_C|SetActivated? _array_element false)
        (Default|DoInteract (Variables|BP_PlatformButton_C|GetMovingPlatformReference _array_element))
        (Math|Integer|IncrementInt (Variables|Default|GetResetCount)))))
  (Development|PrintString (Utilities|String|Append "Reset Loop Completed: Reset count = " (Utilities|String|ToString(Integer) (Variables|Default|GetResetCount)))))