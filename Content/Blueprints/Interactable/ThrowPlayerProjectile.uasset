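; Projectile that stands in for the second player while thrown, turning back into a playable small character on impact.
; On begin play it becomes that player's view target and stores its starting rotation.
; Hitting an actor with "Tall" in its name plays a splat sound and squish animation, then waits briefly.
; Any hit spawns BP_SmallCharacter at the sphere with the starting roll and yaw, possesses it and destroys the projectile.
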(event EventBeginPlay
  (Game|Player|SetViewTargetwithBlend (Game|GetPlayerController 1) self 0.0 "VTBlend_Linear" 0.0 false)
  (Variables|Default|SetStartRotation (Transformation|GetActorRotation self)))

(event Collision|EventHit
  (params (MyComp :type Primitive%20Component%20Object%20Reference) (Other :type Actor%20Object%20Reference) (OtherComp :type Primitive%20Component%20Object%20Reference) (bSelfMoved :type Boolean) (HitLocation :type Vector :default "0, 0, 0") (HitNormal :type Vector :default "0, 0, 0") (NormalImpulse :type Vector :default "0, 0, 0") (Hit :type Hit%20Result%20Structure%20%28by%20ref%29))
  (bind _returnvalue (Utilities|GetDisplayName Other))
  (bind _startrotation (Variables|Default|GetStartRotation))
  (bind _returnvalue_2 (Utilities|String|Contains _returnvalue "Tall"))
  (if _returnvalue_2
    (Development|PrintString (Utilities|String|ToString(Boolean) _returnvalue_2))
    (Audio|PlaySound2D "/Game/Audio/SplatSound.SplatSound" 1.0 1.0 0.0 0 0)
    (Components|Animation|PlayAnimation (Variables|Default|GetSkeletalMesh) "/Game/Animations/LittleCharacter/Little_Squish.Little_Squish" false)
    (Utilities|FlowControl|Delay 0.5))
  (bind _returnvalue_3 (Game|SpawnActorfromClass "/Game/Characters/Players/SmallCharacter/BP_SmallCharacter.BP_SmallCharacter_C" (Math|Transform|MakeTransform (Transformation|GetWorldLocation (Variables|Default|GetSphere1)) (Math|Rotator|MakeRotator (.roll _startrotation) 0.0 (.yaw _startrotation))) "AdjustIfPossibleButDontSpawnIfColliding" 0 0))
  (Pawn|Possess (Game|GetPlayerController 1) _returnvalue_3)
  (Actor|DestroyActor) ; Then destroy this projectile
)

(fn ConstructionScript)