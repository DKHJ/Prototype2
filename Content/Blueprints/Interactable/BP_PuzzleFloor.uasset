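; BP_PuzzleFloor is one floor node in a grid-style movement puzzle, linked to left, right, up and down neighbor nodes.
; TryMoveLeft, TryMoveRight, TryMoveUp and TryMoveDown report whether the neighbor in that direction has IsOpen set, without moving anything themselves.
; Getters expose the four neighbor references, and on BeginPlay the node writes its Index to a text render label.
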(event EventBeginPlay
  (CallFunction|PostInitialise))

(fn ConstructionScript)

(fn PostInitialise
  (Rendering|Components|TextRender|SetText (Variables|Default|GetTextRender) (Utilities|Text|ToText(Integer) (Variables|Default|GetIndex))))

(fn TryMoveLeft
  (bind _newparam (CallFunction|GetNextLeftNode))
  (if (Variables|BP_PuzzleFloor_C|GetIsOpen? _newparam)
    (return true)
    (else
      (return false))))

(fn GetNextLeftNode
  (return (Variables|NodeInfo|GetNextLeftNode)))

(fn GetNextRightNode
  (return (Variables|NodeInfo|GetNextRightNode)))

(fn TryMoveRight
  (bind _nextrightnode (CallFunction|GetNextRightNode))
  (if (Variables|BP_PuzzleFloor_C|GetIsOpen? _nextrightnode)
    (return true)
    (else
      (return false))))

(fn TryMoveUp
  (bind _nextupnode (CallFunction|GetNextUpNode))
  (if (Variables|BP_PuzzleFloor_C|GetIsOpen? _nextupnode)
    (return true)
    (else
      (return false))))

(fn TryMoveDown
  (bind _nextdownnode (CallFunction|GetNextDownNode))
  (if (Variables|BP_PuzzleFloor_C|GetIsOpen? _nextdownnode)
    (return true)
    (else
      (return false))))

(fn GetNextUpNode
  (return (Variables|NodeInfo|GetNextUpNode)))

(fn GetNextDownNode
  (return (Variables|NodeInfo|GetNextDownNode)))