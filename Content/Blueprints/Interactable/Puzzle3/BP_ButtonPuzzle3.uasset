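; Interactable button for Puzzle 3 that only the small character can use.
; Entering its box shows an interact prompt and registers the button with that character via UpdateInteract, and leaving hides the prompt and unregisters it.
; DoInteract plays a button-press montage on the stored character and forwards the interaction to the referenced puzzle actor.
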(event OnComponentBeginOverlap(Box)
  (params (OverlappedComponent :type Primitive%20Component%20Object%20Reference) (OtherActor :type Actor%20Object%20Reference) (OtherComp :type Primitive%20Component%20Object%20Reference) (OtherBodyIndex :type Integer) (bFromSweep :type Boolean) (SweepResult :type Hit%20Result%20Structure%20%28by%20ref%29))
  ;[0 1 0.914] Overlap events
  (bind _asbp_small_character (Utilities|Casting|CastToBP_SmallCharacter OtherActor))
  (Variables|Default|SetSmallCharacterReference _asbp_small_character)
  (Rendering|SetVisibility (Variables|Default|GetInteractText) true false)
  (Default|UpdateInteract _asbp_small_character self true))

(event OnComponentEndOverlap(Box)
  (params (OverlappedComponent :type Primitive%20Component%20Object%20Reference) (OtherActor :type Actor%20Object%20Reference) (OtherComp :type Primitive%20Component%20Object%20Reference) (OtherBodyIndex :type Integer))
  ;[0 1 0.914] Overlap events
  (bind _asbp_small_character (Utilities|Casting|CastToBP_SmallCharacter OtherActor))
  (Rendering|SetVisibility (Variables|Default|GetInteractText) false false)
  (Default|UpdateInteract _asbp_small_character self false))

(event EventDoInteract
  (Animation|PlayAnimMontage (Variables|Default|GetSmallCharacterReference) "/Game/Animations/LittleCharacter/Little_ButtonMont.Little_ButtonMont" 1.0 "None")
  (Default|DoInteract (Variables|Default|GetPuzzleReference)))

(fn ConstructionScript)